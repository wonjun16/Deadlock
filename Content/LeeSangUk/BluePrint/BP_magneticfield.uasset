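; Battle royale style magnetic field actor whose sphere rescales once a countdown expires.
; BeginPlay places it at a small random X/Z location; Tick decrements RemainTime, then plays a Timeline driving the sphere's scale.
; Sphere overlaps print the actor and toggle a single Damage flag, true on exit, which a looping timer checks.
; The health reduction and countdown widget updates are unconnected, so neither runs.
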(event `self.ReceiveBeginPlay`
  (`KismetSystemLibrary.K2_SetTimer` null "Set Hp" 0.5 true)
  (`self.K2_SetActorLocation` self (`KismetMathLibrary.MakeVector` (`KismetMathLibrary.RandomFloatInRange` -10.0 10.0) 0.0 (`KismetMathLibrary.RandomFloatInRange` -10.0 10.0)) false false))

(event `self.ReceiveTick`
  (params (DeltaSeconds :type "Float (single-precision)"))
  (`self.CheckRemainTime` DeltaSeconds)
  (if (<= (`self.RemainTime`) 0.0)
    (bind (_direction _newtrack_0) (`Timeline|Timeline`)
      (:`Update`
        (`SceneComponent.SetWorldScale3D` (`self.Sphere`) (`KismetMathLibrary.Conv_DoubleToVector` _newtrack_0))))))

(event `self.Sphere.OnComponentBeginOverlap`
  (params (OverlappedComponent :type "PrimitiveComponent Object Reference") (OtherActor :type "Actor Object Reference") (OtherComp :type "PrimitiveComponent Object Reference") (OtherBodyIndex :type Integer) (bFromSweep :type Boolean) (SweepResult :type "HitResult Structure (by ref)"))
  (`KismetSystemLibrary.PrintString` (`KismetSystemLibrary.GetDisplayName` OtherActor))
  (set `self.Damage` false))

(event `self.Sphere.OnComponentEndOverlap`
  (params (OverlappedComponent :type "PrimitiveComponent Object Reference") (OtherActor :type "Actor Object Reference") (OtherComp :type "PrimitiveComponent Object Reference") (OtherBodyIndex :type Integer))
  (`KismetSystemLibrary.PrintString` (`KismetStringLibrary.Concat_StrStr` "End : " (`KismetSystemLibrary.GetDisplayName` OtherActor)))
  (set `self.Damage` true))

(fn `CheckRemainTime`
  (params (TeltaTime :type "Float (double-precision)"))
  (set `self.RemainTime` (- (`self.RemainTime`) TeltaTime)))

(fn `Set Hp`
  (if (`self.Damage`)
    _))

(fn `UserConstructionScript`)