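; BP_DeadlockCharacter123 is a character Blueprint holding only disconnected item-throwing logic, so it runs no behavior of its own.
; Its unreachable main chain waits, then searches placed ItemBase actors for the player state's selected item type.
; It spawns that class at the LeftHand socket and, for certain types, calls ThrowMovement along the actor's forward vector.
; BeginPlay and the construction script are empty, alongside stray enum-iteration and weapon-socket nodes.
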(event `self.ReceiveBeginPlay`)

(fn `UserConstructionScript`)